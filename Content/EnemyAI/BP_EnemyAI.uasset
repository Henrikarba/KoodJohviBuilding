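; BP_EnemyAI is a zombie enemy with health, sight and a melee attack against the player.
; Seeing a pawn through PawnSensing sets a seen flag on the AI controller's Blackboard.
; MeeleAttack starts the attack montage and immediately sphere-traces a short distance forward for pawns, applying damage to the one hit.
; Incoming damage lowers clamped health; at zero it calls Killed on AI_Controller, then destroys the actor.
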(event OnSeePawn(PawnSensing)
  (params (Pawn :type Pawn%20Object%20Reference))
  (AI|Components|Blackboard|SetValueasBool (AI|GetBlackboard (AI|GetAIController self)) (Variables|Default|GetSeen%20Key%20Name) true))

(event Custom|Meele%20Attack
  (bind _returnvalue (Transformation|GetActorLocation))
  ;[1 1 1] Attack Player
  (Animation|Montage|PlayMontage (Variables|Character|GetMesh) "/Game/EnemyAI/TposeZombie1/Animations/zombie_attack1.zombie_attack1"
    (:then
      (bind (_outhit _returnvalue_2) (Collision|SphereTraceForObjects _returnvalue (+ _returnvalue (* (Math|Vector|GetForwardVector (Transformation|GetActorRotation)) 1.2e+02)) 3e+01 (Utilities|Array|MakeArray "ObjectTypeQuery3") false 0 "None"))
      (if _returnvalue_2
        (Game|Damage|ApplyDamage (.HitActor (Collision|BreakHitResult _outhit)) (Variables|Default|GetDamage%20To%20Player) 0 self)))))

(event Game|Damage|EventAnyDamage
  (params (Damage :type Float%20%28single-precision%29) (DamageType :type Damage%20Type%20Object%20Reference) (InstigatedBy :type Controller%20Object%20Reference) (DamageCauser :type Actor%20Object%20Reference))
  ;[1 1 1] Take Damage
  (bind _output_get (Variables|Default|SetHealth (Math|Float|Clamp(Float) (- (Variables|Default|GetHealth) Damage) 0.0 (Variables|Default|GetMax%20Health))))
  (if (== _output_get 0.0)
    (bind _asai_controller (Utilities|Casting|CastToAI_Controller (Pawn|GetController)))
    (Default|Killed _asai_controller)
    (Actor|DestroyActor)))

(fn ConstructionScript)